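; BP_HealthPickup1 is an interactable health pickup for the first-person character.
; On Interact, if the character's Health is below 100, it passes itself, HealthAmount, the Infinite flag and current Health to CPPInventory's HealthPickup function, then writes the returned value back as Health.
; GetInteractInfo reports an instant interaction with no hold time.
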(event `self.ReceiveTick`
  (params (DeltaSeconds :type "Float (single-precision)")))

(event `/Game/Inventory/InteractInterface.Interact`
  (params (Interactor :type "Actor Object Reference"))
  (bind _asfirst_person_character (cast `/Game/FirstPersonBP/Blueprints/FirstPersonCharacter` Interactor))
  ;[1 1 1] Player doesn't have max ammo
  (if (< (`/Game/FirstPersonBP/Blueprints/FirstPersonCharacter.Health` _asfirst_person_character) 100.0)
    (bind _outhealth (`CPPInventory.HealthPickup` (`self.CPPInventory`) self (`self.HealthAmount`) (`self.Infinite`) (`/Game/FirstPersonBP/Blueprints/FirstPersonCharacter.Health` _asfirst_person_character)))
    (set `/Game/FirstPersonBP/Blueprints/FirstPersonCharacter.Health` _outhealth _asfirst_person_character)))

(fn `Get Interact Info`
  (params (Interactor :type "/Game/FirstPersonBP/Blueprints/FirstPersonCharacter Object Reference"))
  (returns (`Held Interact` :type Boolean) (`Interact Time` :type "Float (double-precision)"))
  (return false 0.0))

(fn `UserConstructionScript`)