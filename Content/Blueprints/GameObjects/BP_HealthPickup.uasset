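; BP_HealthPickup is an interactable health pickup that restores health to a first-person character.
; On Interact it only acts if the player's health is below 100, then passes itself, the heal amount and infinite flag to the player's Inventory component.
; A Switch Has Authority chooses the server or client pickup call, and the interaction is instant rather than held.
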(event `self.ReceiveTick`
  (params (DeltaSeconds :type "Float (single-precision)")))

(event `/Game/Inventory/InteractInterface.Interact`
  (params (Interactor :type "Actor Object Reference"))
  (bind _healthamount (`self.HealthAmount`))
  (bind _infinite (`self.Infinite`))
  (bind _asfirst_person_character (cast `/Game/FirstPersonBP/Blueprints/FirstPersonCharacter` Interactor))
  ;[1 1 1] Player doesn't have max ammo
  (if (< (`/Game/FirstPersonBP/Blueprints/FirstPersonCharacter.Health` _asfirst_person_character) 100.0)
    (`/Engine/EditorBlueprintResources/ActorMacros.Switch Has Authority`
      (:`Authority`
        (bind _inventory (`/Game/FirstPersonBP/Blueprints/FirstPersonCharacter.Inventory` _asfirst_person_character))
        (`/Game/Inventory/Inventory.HealthPickup` _inventory self _healthamount _infinite _asfirst_person_character))
      (:`Remote`
        (`/Game/Inventory/Inventory.HealthPickupClient` _inventory self _healthamount _infinite _asfirst_person_character)))))

(fn `Get Interact Info`
  (params (Interactor :type "/Game/FirstPersonBP/Blueprints/FirstPersonCharacter Object Reference"))
  (returns (`Held Interact` :type Boolean) (`Interact Time` :type "Float (double-precision)"))
  (return false 0.0))

(fn `UserConstructionScript`)