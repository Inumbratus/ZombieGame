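; Sliding door actor that opens while a Pawn is inside its Box trigger and closes when none remain.
; Begin overlap sets Open, and end overlap rechecks the remaining overlapping actors through TestForPlayers.
; Tick steps the Cube up, right or left toward MovementMax or back to zero by Speed per frame, without delta-time scaling.
; Locked halts all movement, though overlaps still update Open.
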(event `self.ReceiveTick`
  (params (DeltaSeconds :type "Float (single-precision)"))
  (bind _cube (`self.Cube`))
  (bind _speed (`self.Speed`))
  (bind _cube_2 (`self.Cube`))
  (bind _speed_2 (`self.Speed`))
  (bind _movementmax (`self.MovementMax`))
  (bind (_relativelocation_x _relativelocation_y _relativelocation_z) (`KismetMathLibrary.BreakVector` (`SceneComponent.RelativeLocation` (`self.Cube`))))
  (bind (_relativelocation_x_2 _relativelocation_y_2 _relativelocation_z_2) (`KismetMathLibrary.BreakVector` (`SceneComponent.RelativeLocation` (`self.Cube`))))
  (if (`self.Locked`)
    _
    (elif (`self.Open`)
      (switch `/Game/Blueprints/GameObjects/Enum_DoorSliding` (`self.SlideDirection`)
        (:`NewEnumerator0`
          (if (< _relativelocation_z_2 _movementmax)
            (`SceneComponent.K2_AddRelativeLocation` _cube_2 (`KismetMathLibrary.MakeVector` 0.0 0.0 _speed_2) false false)))
        (:`NewEnumerator1`
          (if (< _relativelocation_x_2 _movementmax)
            (`SceneComponent.K2_AddRelativeLocation` _cube_2 (`KismetMathLibrary.MakeVector` _speed_2) false false)))
        (:`NewEnumerator2`
          (if (> _relativelocation_x_2 (* _movementmax -1.0))
            (`SceneComponent.K2_AddRelativeLocation` _cube_2 (`KismetMathLibrary.MakeVector` (* _speed_2 -1.0)) false false))))
      (else
        (switch `/Game/Blueprints/GameObjects/Enum_DoorSliding` (`self.SlideDirection`)
          (:`NewEnumerator0`
            (if (> _relativelocation_z 0.0)
              (`SceneComponent.K2_AddRelativeLocation` _cube (`KismetMathLibrary.MakeVector` 0.0 0.0 (* _speed -1.0)) false false)))
          (:`NewEnumerator1`
            (if (> _relativelocation_x 0.0)
              (`SceneComponent.K2_AddRelativeLocation` _cube (`KismetMathLibrary.MakeVector` (* _speed -1.0)) false false)))
          (:`NewEnumerator2`
            (if (< _relativelocation_x 0.0)
              (`SceneComponent.K2_AddRelativeLocation` _cube (`KismetMathLibrary.MakeVector` _speed) false false))))))))

(event `self.Box.OnComponentBeginOverlap`
  (params (OverlappedComponent :type "PrimitiveComponent Object Reference") (OtherActor :type "Actor Object Reference") (OtherComp :type "PrimitiveComponent Object Reference") (OtherBodyIndex :type Integer) (bFromSweep :type Boolean) (SweepResult :type "HitResult Structure (by ref)"))
  (cast `Pawn` OtherActor)
  (set `self.Open` true))

(event `self.Box.OnComponentEndOverlap`
  (params (OverlappedComponent :type "PrimitiveComponent Object Reference") (OtherActor :type "Actor Object Reference") (OtherComp :type "PrimitiveComponent Object Reference") (OtherBodyIndex :type Integer))
  (bind _ischaracter1 (`self.TestForPlayers`))
  (set `self.Open` _ischaracter1))

(fn `TestForPlayers`
  (returns (isCharacter1 :type Boolean))
  (locals (isCharacter :type Boolean))
  (for _array_element (`PrimitiveComponent.GetOverlappingActors` (`self.Box`) null)
    (cast `Pawn` _array_element)
    (set `local.isCharacter` true))
  (return (`local.isCharacter`)))

(fn `UserConstructionScript`)