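; BP_AmmoPickup1 is an interactable ammo pickup that refills reserve ammo for the first-person character's equipped weapon on an instant, non-held interact.
; Interact only proceeds when the weapon's combined magazine and reserve ammo is below its combined capacity.
; It passes itself, its amount, its Infinite flag and the weapon specs to CPPInventory's AmmoPickup, then writes the result into the weapon's reserve ammo.
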(event `self.ReceiveTick`
  (params (DeltaSeconds :type "Float (single-precision)")))

(event `/Game/Inventory/InteractInterface.Interact`
  (params (Interactor :type "Actor Object Reference"))
  (bind _asfirst_person_character (cast `/Game/FirstPersonBP/Blueprints/FirstPersonCharacter` Interactor))
  (bind (_basedamage _roundsperburst _range _verticalrecoilvariation _horizontalrecoilvariation _recoilprofile _reloadspeed _firerate _spread _magazinesize _magazineammo _reserveammo _maxreserveammo) (break `/Game/Inventory/WeaponSpecs` (`.WeaponSpecs_89_498B50AF4A0DD1F107347F8D2FB6A0D0` (break `/Game/Inventory/Weapon` (`/Game/Inventory/Inventory.EquippedWeapon` (`/Game/FirstPersonBP/Blueprints/FirstPersonCharacter.Inventory` _asfirst_person_character))))))
  ;[1 1 1] Player doesn't have max ammo
  (if (< (+ _magazineammo _reserveammo) (+ _magazinesize _maxreserveammo))
    (bind _outammo (`CPPInventory.AmmoPickup` (`self.CPPInventory`) self (`self.AmmoAmount`) (`self.Infinite`) _magazinesize _magazineammo _reserveammo _maxreserveammo))
    (`|VariableSetRef` _reserveammo _outammo)))

(fn `Get Interact Info`
  (params (Interactor :type "/Game/FirstPersonBP/Blueprints/FirstPersonCharacter Object Reference"))
  (returns (`Held Interact` :type Boolean) (`Interact Time` :type "Float (double-precision)"))
  (return false 0.0))

(fn `UserConstructionScript`)