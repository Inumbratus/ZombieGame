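; Interactable, lockable door that toggles open and closed on instant interaction, sliding its mesh vertically.
; A FlipFlop plays or reverses the OpenDoor timeline, which lowers the mesh from the position captured on opening.
; A DoOnce starts a looping sound at the frame while the timeline moves and stops it on finish.
; Two point lights show when it starts locked; Unlock clears the lock and turns their colour black.
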(event `/Game/Inventory/InteractInterface.Interact`
  (params (Interactor :type "Actor Object Reference"))
  (bind (_def_x _def_y _def_z) (`KismetMathLibrary.BreakVector` (`self.Def`)))
  (bind _audio (`self.Audio`))
  ;[1 1 1 1 45] Door function
  (if (not (`self.Locked`))
    (`/Engine/EditorBlueprintResources/StandardMacros.FlipFlop`
      (:`A`
        (set `self.Def` (`SceneComponent.RelativeLocation` (`self.StaticMesh`)))
        (bind (_direction _dooropening) (`Timeline|OpenDoor` :!label _label)
          (:`Update`
            (`|ExecutionSequence`
              (:`then_0`
                (`SceneComponent.K2_SetRelativeLocation` (`self.StaticMesh`) (`KismetMathLibrary.MakeVector` _def_x _def_y (- _def_z _dooropening)) false false))
              (:`then_1`
                (`/Engine/EditorBlueprintResources/StandardMacros.DoOnce` false :!label _label_2
                  (:`Completed`
                    (`/Engine/EditorBlueprintResources/StandardMacros.IsValid` _audio
                      (:`Is Valid`
                        (`AudioComponent.Stop` _audio))
                      (:`Is Not Valid`
                        _))
                    ;;[1 1 1] Add sounds
                    (bind _returnvalue (`GameplayStatics.SpawnSoundAtLocation` "/Game/Assets/Sound/EnviromentSounds/DoorClosingLoop.DoorClosingLoop" (`SceneComponent.K2_GetComponentLocation` (`self.DoorFrame`)) (struct) 0.5 0.8 0.0 "/Game/Audio/AT_door.AT_door" null))
                    (set `self.Audio` _returnvalue))))))
          (:`Finished`
            (`AudioComponent.Stop` (`self.Audio`))
            (goto _label_2 :!via `Reset`))))
      (:`B`
        (goto _label :!via `Reverse`)))))

(event `/Game/Inventory/InteractInterface.Unlock`
  ;[1 1 1 1 45] Door function
  (set `self.Locked` false)
  (`LightComponent.SetLightColor` :`self` (`self.PointLight`))
  (`LightComponent.SetLightColor` :`self` (`self.PointLight1`)))

(event `self.ReceiveBeginPlay`
  ;[1 1 1] Debugs
  (if (`self.Locked`)
    (`SceneComponent.SetVisibility` (`self.PointLight`) true false)
    (`SceneComponent.SetVisibility` (`self.PointLight1`) true false)))

(event `Key|Q`
  (params (Key :type "Key Structure"))
  ;[1 1 1] Debugs
)

(fn `Get Interact Info`
  (params (Interactor :type "/Game/FirstPersonBP/Blueprints/FirstPersonCharacter Object Reference"))
  (returns (`Held Interact` :type Boolean) (`Interact Time` :type "Float (double-precision)"))
  (return false 0.0))

(fn `UserConstructionScript`)