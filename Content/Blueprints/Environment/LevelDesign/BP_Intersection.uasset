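; BP_Intersection is a level design intersection piece with four wall meshes that are set up in the construction script.
; Randomise gives each wall a random mesh from the SMWallReferences array every time construction runs.
; HideWalls then uses the BWallX and BWallY flags to show or hide the walls in pairs, turning off collision on hidden ones.
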(fn `Hide Walls`
  (params (Condition :type Boolean) (`SM Component` :type "PrimitiveComponent Object Reference"))
  (if Condition
    (`SceneComponent.SetVisibility` `SM Component` true false)
    (else
      (`SceneComponent.SetVisibility` `SM Component` false false)
      (`PrimitiveComponent.SetCollisionEnabled` `SM Component` "NoCollision"))))

(fn `Randomise`
  (bind _sm_wall_references (`self.SM_Wall_References`))
  (bind _output (`|GetArrayItem` _sm_wall_references (`KismetMathLibrary.RandomInteger` (`KismetArrayLibrary.Array_Length` _sm_wall_references))))
  (`StaticMeshComponent.SetStaticMesh` (`self.StaticMesh4`) _output)
  (`StaticMeshComponent.SetStaticMesh` (`self.StaticMesh2`) _output)
  (`StaticMeshComponent.SetStaticMesh` (`self.StaticMesh5`) _output)
  (`StaticMeshComponent.SetStaticMesh` (`self.StaticMesh3`) _output))

(fn `UserConstructionScript`
  (`self.Randomise`)
  (`self.Hide Walls` (`self.b_Wall_X+`) (`self.StaticMesh3`))
  (`self.Hide Walls` (`self.b_Wall_Y+`) (`self.StaticMesh2`))
  (`self.Hide Walls` (`self.b_Wall_Y-`) (`self.StaticMesh4`))
  (`self.Hide Walls` (`self.b_Wall_X-`) (`self.StaticMesh5`)))