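; Level-design sliding door for the fingerprint puzzle area that opens when a Pawn enters its trigger volume.
; A timeline lerps the door mesh between closed and open positions, with steam activated on entry and a replaceable looping sound at the door.
; On Pawn exit, the timeline reverses at a higher sound pitch only if TestForPlayers returns true from its scan of Pawns overlapping the trigger.
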(event `self.Trigger.OnComponentBeginOverlap`
  (params (OverlappedComponent :type "PrimitiveComponent Object Reference") (OtherActor :type "Actor Object Reference") (OtherComp :type "PrimitiveComponent Object Reference") (OtherBodyIndex :type Integer) (bFromSweep :type Boolean) (SweepResult :type "HitResult Structure (by ref)"))
  (bind _audio (`self.Audio`))
  (cast `Pawn` OtherActor)
  (`ActorComponent.Activate` (`self.SteamDoor`) false)
  (`ActorComponent.Activate` (`self.SteamDoor2`) false)
  (`/Engine/EditorBlueprintResources/StandardMacros.IsValid` _audio
    (:`Is Valid`
      (`AudioComponent.Stop` _audio))
    (:`Is Not Valid`
      _))
  (bind _returnvalue (`GameplayStatics.SpawnSoundAtLocation` "/Game/Assets/Sound/EnviromentSounds/DoorClosingLoop.DoorClosingLoop" (`SceneComponent.K2_GetComponentLocation` (`self.Door_Small_A`)) (struct) 0.5 0.5 0.0 "/Game/Audio/AT_door.AT_door" null))
  (set `self.Audio` _returnvalue)
  (bind (_direction _doorposition) (`Timeline|Timeline_0` :!label _label)
    (:`Update`
      (`SceneComponent.K2_SetRelativeLocation` (`self.Door_Small_A`) (`KismetMathLibrary.VLerp` (`self.DoorClosed`) (`self.DoorOpen`) _doorposition) false false))
    (:`Finished`
      (`AudioComponent.Stop` (`self.Audio`)))))

(event `self.Trigger.OnComponentEndOverlap`
  (params (OverlappedComponent :type "PrimitiveComponent Object Reference") (OtherActor :type "Actor Object Reference") (OtherComp :type "PrimitiveComponent Object Reference") (OtherBodyIndex :type Integer))
  (bind _audio (`self.Audio`))
  (cast `Pawn` OtherActor)
  (bind _ischaracter1 (`self.TestForPlayers`))
  (if _ischaracter1
    (`/Engine/EditorBlueprintResources/StandardMacros.IsValid` _audio
      (:`Is Valid`
        (`AudioComponent.Stop` _audio))
      (:`Is Not Valid`
        _))
    (bind _returnvalue (`GameplayStatics.SpawnSoundAtLocation` "/Game/Assets/Sound/EnviromentSounds/DoorClosingLoop.DoorClosingLoop" (`SceneComponent.K2_GetComponentLocation` (`self.Door_Small_A`)) (struct) 0.5 0.8 0.0 "/Game/Audio/AT_door.AT_door" null))
    (set `self.Audio` _returnvalue)
    (goto _label :!via `Reverse`)))

(fn `TestForPlayers`
  (returns (isCharacter1 :type Boolean))
  (locals (isCharacter :type Boolean))
  (for _array_element (`PrimitiveComponent.GetOverlappingActors` (`self.Trigger`) null)
    (cast `Pawn` _array_element)
    (set `local.isCharacter` true))
  (return (`local.isCharacter`)))

(fn `UserConstructionScript`)